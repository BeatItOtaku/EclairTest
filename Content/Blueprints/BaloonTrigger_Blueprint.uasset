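; BaloonTrigger is a one-shot trigger volume that shows a timed speech balloon UI with configurable text.
; When something overlaps its Box while enabled, it creates a PersonBaloonUI widget, plays its In animation and disables itself.
; After the Duration delay it plays the Out animation, without removing the widget itself.
; The construction script sizes the Box from the Extent variable.
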(event `self.Box.OnComponentBeginOverlap`
  (params (OverlappedComponent :type "PrimitiveComponent Object Reference") (OtherActor :type "Actor Object Reference") (OtherComp :type "PrimitiveComponent Object Reference") (OtherBodyIndex :type Integer) (bFromSweep :type Boolean) (SweepResult :type "HitResult Structure (by ref)"))
  (bind _uireference (`self.UIReference`))
  (bind _uireference_2 (`self.UIReference`))
  (if (`self.Enabled`)
    (bind _returnvalue (`|CreateWidget` "/Game/UI/PersonBaloonUI.PersonBaloonUI_C" null (`self.Text`)))
    (bind _output_get (set `self.UIReference` _returnvalue))
    (`UserWidget.AddToViewport` _output_get 0)
    (`UserWidget.PlayAnimation` _uireference_2 (`/Game/UI/PersonBaloonUI.In` _uireference_2) 0.0 1 "Forward" 1.0)
    (set `self.Enabled` false)
    (`KismetSystemLibrary.Delay` (`self.Duration`))
    (`UserWidget.PlayAnimation` _uireference (`/Game/UI/PersonBaloonUI.Out` _uireference) 0.0 1 "Forward" 1.0)))

(fn `UserConstructionScript`
  (`BoxComponent.SetBoxExtent` (`self.Box`) (`self.Extent`) true))