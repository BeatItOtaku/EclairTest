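; Kama actor that turns toward and glides to an anchor point in the level.
; BeginPlay collects and prints the world locations of all Kama_Anchor_Blueprint actors into an array.
; Each Tick snaps rotation to face the indexed location and eases toward it with VInterpTo, without sweeping.
; The index increment is unconnected, so this graph never advances to another anchor.
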(event `self.ReceiveBeginPlay`
  (bind _outactors (`GameplayStatics.GetAllActorsOfClass` "/Game/Blueprints/Kama_Anchor_Blueprint.Kama_Anchor_Blueprint_C"))
  (for _array_element _outactors
    (bind _askama_anchor_blueprint (cast `/Game/Blueprints/Kama_Anchor_Blueprint` _array_element))
    (bind _returnvalue (`SceneComponent.K2_GetComponentLocation` (`Actor.RootComponent` _askama_anchor_blueprint)))
    (`KismetArrayLibrary.Array_Add` (`self.AnchorLocations`) _returnvalue)
    (`KismetSystemLibrary.PrintString` (`KismetStringLibrary.Conv_VectorToString` _returnvalue))))

(event `self.ReceiveTick`
  (params (DeltaSeconds :type "Float (single-precision)"))
  (bind _returnvalue (`self.K2_GetActorLocation`))
  (bind _output (`|GetArrayItem` (`self.AnchorLocations`) (`self.ArrayIndex`)))
  (`self.K2_SetActorRotation` (`KismetMathLibrary.FindLookAtRotation` _returnvalue _output)) ; 釜がアンカーの方を向く
  (`self.K2_SetActorLocation` (`KismetMathLibrary.VInterpTo` _returnvalue _output (`GameplayStatics.GetWorldDeltaSeconds`) 0.5)) ; 釜がアンカーに移動する移動させる
)

(fn `UserConstructionScript`)