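; HiRaishin is an actor with a sphere collider that flags overlapping ThirdPersonCharacters as ETO-jammed.
; BeginPlay sizes the collider from SphereRadius, and both begin and end overlap call EtoJammer, then print a debug message.
; EtoJammer sets ETOJammered to true and stores the mesh's location as the character's JammingSpot.
; An optional SwitchActor gates the effect through SwitchOn; without a valid one, jamming always applies.
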(event `self.ReceiveBeginPlay`
  (`SphereComponent.SetSphereRadius` (`self.Collider`) (`self.SphereRadius`) true))

(event `self.ReceiveTick`
  (params (DeltaSeconds :type "Float (single-precision)")))

(event `self.Collider.OnComponentBeginOverlap`
  (params (OverlappedComponent :type "PrimitiveComponent Object Reference") (OtherActor :type "Actor Object Reference") (OtherComp :type "PrimitiveComponent Object Reference") (OtherBodyIndex :type Integer) (bFromSweep :type Boolean) (SweepResult :type "HitResult Structure (by ref)"))
  (`self.EtoJammer` OtherActor)
  (`KismetSystemLibrary.PrintString` "Jamming" :!label _label))

(event `self.Collider.OnComponentEndOverlap`
  (params (OverlappedComponent :type "PrimitiveComponent Object Reference") (OtherActor :type "Actor Object Reference") (OtherComp :type "PrimitiveComponent Object Reference") (OtherBodyIndex :type Integer))
  (`self.EtoJammer` OtherActor)
  (goto _label))

(fn `EtoJammer`
  (params (Actor :type "Actor Object Reference"))
  (`/Engine/EditorBlueprintResources/StandardMacros.IsValid` (`self.SwitchActor`)
    (:`Is Valid`
      (if (`/Game/Blueprints/SwitchActor_Blueprint.SwitchOn` (`self.SwitchActor`))
        (bind _asthird_person_character (cast `/Game/ThirdPersonBP/Blueprints/ThirdPersonCharacter` Actor :!label _label))
        (set `/Game/ThirdPersonBP/Blueprints/ThirdPersonCharacter.ETOJammered` true _asthird_person_character)
        (set `/Game/ThirdPersonBP/Blueprints/ThirdPersonCharacter.JammingSpot` (`SceneComponent.K2_GetComponentLocation` (`self.StaticMeshComponent`)) _asthird_person_character)))
    (:`Is Not Valid`
      (goto _label))))

(fn `UserConstructionScript`)