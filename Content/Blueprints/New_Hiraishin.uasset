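; Lightning rod (Hiraishin) actor that jams the ETO state of any ThirdPersonCharacter inside its sphere collider.
; Begin and end overlap set or clear ETOJammered, then both call EtoJammer and print a debug message.
; EtoJammer runs if no SwitchActor is valid or it is on.
; It stores the jamming center and player offset, turns the player toward the center, and derives HiraishinAxis by rotating that direction 90 degrees.
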(event `self.ReceiveBeginPlay`
  (`SphereComponent.SetSphereRadius` (`self.Collider`) (`self.SphereRadius`) true))

(event `self.Collider.OnComponentBeginOverlap`
  (params (OverlappedComponent :type "PrimitiveComponent Object Reference") (OtherActor :type "Actor Object Reference") (OtherComp :type "PrimitiveComponent Object Reference") (OtherBodyIndex :type Integer) (bFromSweep :type Boolean) (SweepResult :type "HitResult Structure (by ref)"))
  (bind _asthird_person_character (cast `/Game/ThirdPersonBP/Blueprints/ThirdPersonCharacter` OtherActor))
  (set `self.Player` _asthird_person_character)
  (set `/Game/ThirdPersonBP/Blueprints/ThirdPersonCharacter.ETOJammered` true (`self.Player`))
  (`self.EtoJammer` (`self.Player`))
  (`KismetSystemLibrary.PrintString` "Jamming" :!label _label))

(event `self.Collider.OnComponentEndOverlap`
  (params (OverlappedComponent :type "PrimitiveComponent Object Reference") (OtherActor :type "Actor Object Reference") (OtherComp :type "PrimitiveComponent Object Reference") (OtherBodyIndex :type Integer))
  (bind _asthird_person_character (cast `/Game/ThirdPersonBP/Blueprints/ThirdPersonCharacter` OtherActor))
  (set `self.Player` _asthird_person_character)
  (set `/Game/ThirdPersonBP/Blueprints/ThirdPersonCharacter.ETOJammered` false (`self.Player`))
  (`self.EtoJammer` (`self.Player`))
  (goto _label))

(fn `EtoJammer`
  (params (Actor :type "Actor Object Reference"))
  (bind _player (`self.Player`))
  (bind _player_2 (`self.Player`))
  (bind _returnvalue (`SceneComponent.K2_GetComponentLocation` (`Actor.RootComponent` _player)))
  (`/Engine/EditorBlueprintResources/StandardMacros.IsValid` (`self.SwitchActor`)
    (:`Is Valid`
      (if (`/Game/Blueprints/SwitchActor_Blueprint.SwitchOn` (`self.SwitchActor`))
        (bind _output_get (set `/Game/ThirdPersonBP/Blueprints/ThirdPersonCharacter.JammingSpot` (`SceneComponent.K2_GetComponentLocation` (`self.Collider`)) _player :!label _label))
        (set `/Game/ThirdPersonBP/Blueprints/ThirdPersonCharacter.ETOPosition` (- _returnvalue _output_get) _player_2)
        (`self.K2_SetActorRotation` (`self.Player`) (`KismetMathLibrary.FindLookAtRotation` (`SceneComponent.K2_GetComponentLocation` (`Actor.RootComponent` _player_2)) _output_get) false) ; エクレアを避雷針の中心に向けさせる
        (set `/Game/ThirdPersonBP/Blueprints/ThirdPersonCharacter.HiraishinAxis` (`KismetMathLibrary.GreaterGreater_VectorRotator` (`KismetMathLibrary.Normal` (- _output_get _returnvalue)) (struct :`Yaw` 90.0)) (`self.Player`))))
    (:`Is Not Valid`
      (goto _label))))

(fn `UserConstructionScript`)