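; Pit-style respawn actor (naraku) that moves the player character when it enters the area around the actor.
; Every tick it runs a wide, flat box trace upward on the Visibility channel, with per-frame debug drawing.
; A hit ThirdPersonCharacter is stored as Player, and its root is shifted by RespownPoint.
; RespownPoint acts as a relative world offset, not an absolute destination.
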(event `self.ReceiveTick`
  (params (DeltaSeconds :type "Float (single-precision)"))
  (bind _returnvalue (`self.K2_GetActorLocation`))
  (bind _outhit (`KismetSystemLibrary.BoxTraceSingle` :`Start` _returnvalue :`End` (+ _returnvalue (* (`self.GetActorUpVector`) 100.0)) :`HalfSize` (1000.0 1000.0 100.0) :`TraceChannel` "TraceTypeQuery1" :`DrawDebugType` "ForOneFrame"))
  (bind _asthird_person_character (cast `/Game/ThirdPersonBP/Blueprints/ThirdPersonCharacter` (`.HitActor` (`GameplayStatics.BreakHitResult` _outhit))))
  (bind _output_get (set `self.Player` _asthird_person_character))
  (`SceneComponent.K2_AddWorldOffset` (`Actor.RootComponent` (`self.Player`)) (`self.RespownPoint`) false false))

(fn `UserConstructionScript`)