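; Switch actor whose on state can expire after a limited time, with a box collider tracking whether the ThirdPersonCharacter is in front of it.
; BeginPlay sizes the collider and loads the countdown.
; While the player overlaps, Tick counts down and prints the remaining time if the switch is on, time-limited and not always switchable, then turns it off and resets.
; Nothing in these graphs turns the switch on.
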(event `self.ReceiveBeginPlay`
  (`BoxComponent.SetBoxExtent` (`self.Collider`) (`self.BoxColliderScale`) true)
  (set `self.CurrentTime` (`self.LimitedTime`)))

(event `self.ReceiveTick`
  (params (DeltaSeconds :type "Float (single-precision)"))
  (if (`self.PlayerInFrontOfSwtich`)
    (if (`self.SwitchOn`)
      (if (`self.CanAlwaysSwitch`)
        _
        (elif (`self.UseLimitedTime`)
          (bind _output_get (set `self.CurrentTime` (- (`self.CurrentTime`) (`GameplayStatics.GetWorldDeltaSeconds`))))
          (`KismetSystemLibrary.PrintString` (`KismetStringLibrary.Conv_DoubleToString` _output_get))
          (if (<= _output_get 0.0)
            (set `self.SwitchOn` false)
            (set `self.CurrentTime` (`self.LimitedTime`))))))))

(event `self.Collider.OnComponentBeginOverlap`
  (params (OverlappedComponent :type "PrimitiveComponent Object Reference") (OtherActor :type "Actor Object Reference") (OtherComp :type "PrimitiveComponent Object Reference") (OtherBodyIndex :type Integer) (bFromSweep :type Boolean) (SweepResult :type "HitResult Structure (by ref)"))
  (cast `/Game/ThirdPersonBP/Blueprints/ThirdPersonCharacter` OtherActor)
  (set `self.PlayerInFrontOfSwtich` true))

(event `self.Collider.OnComponentEndOverlap`
  (params (OverlappedComponent :type "PrimitiveComponent Object Reference") (OtherActor :type "Actor Object Reference") (OtherComp :type "PrimitiveComponent Object Reference") (OtherBodyIndex :type Integer))
  (cast `/Game/ThirdPersonBP/Blueprints/ThirdPersonCharacter` OtherActor)
  (set `self.PlayerInFrontOfSwtich` false))

(fn `UserConstructionScript`)