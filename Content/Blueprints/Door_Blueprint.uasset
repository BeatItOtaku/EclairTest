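; Door Blueprint that derives an IsOpen flag from a list of switch actors; no door movement happens here.
; Each Tick multiplies SwitchOnCount by 1 or -1 per switch's SwitchOn state, stopping once it is not positive.
; IsOpen is true when the count stays positive, but the count is never reset between ticks, so it carries over.
; Switch states, IsOpen and the count print for debugging.
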(event `self.ReceiveTick`
  (params (DeltaSeconds :type "Float (single-precision)"))
  (for _array_element (`self.SwitchActors`)
    (bind _switchon (`/Game/Blueprints/SwitchActor_Blueprint.SwitchOn` _array_element))
    (`KismetSystemLibrary.PrintString` (`KismetStringLibrary.Conv_BoolToString` _switchon))
    (bind _output_get (set `self.SwitchOnCount` (* (`self.SwitchOnCount`) (`KismetMathLibrary.SelectInt` 1 -1 _switchon))))
    (if (not (> _output_get 0))
      (break)))
  (bind _output_get_2 (set `self.IsOpen` (> (`self.SwitchOnCount`) 0)))
  (`KismetSystemLibrary.PrintString` (`KismetStringLibrary.Conv_BoolToString` _output_get_2))
  (`KismetSystemLibrary.PrintString` (`KismetStringLibrary.Conv_IntToString` (`self.SwitchOnCount`))))

(fn `UserConstructionScript`)