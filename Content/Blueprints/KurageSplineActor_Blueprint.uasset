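; Spline path actor, named for a jellyfish (kurage), that other objects query to move along its spline by travelled distance.
; GetCurrentLocation converts a distance to a world location, wrapping by the spline length when looping is requested.
; GetLength exposes the total spline length and IsArrived reports whether a distance has reached the end.
; The event graph and construction script hold no logic.
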(fn `GetCurrentLocation`
  (params (Length :type "Float (double-precision)") (Loop :type Boolean))
  (returns (NewParam :type "Vector Structure"))
  (locals (LocalLength :type "Float (double-precision)"))
  (if Loop
    (set `local.LocalLength` (mod Length (`SplineComponent.GetSplineLength` (`self.Spline`)))) ; ループを考慮して剰余から再計算
    (else
      (set `local.LocalLength` Length)))
  (return (`SplineComponent.GetLocationAtDistanceAlongSpline` (`self.Spline`) (`local.LocalLength`) "World")))

(fn `GetLength`
  (returns (Length :type "Float (double-precision)"))
  (return (`SplineComponent.GetSplineLength` (`self.Spline`))))

(fn `IsArrived`
  (params (Length :type "Float (double-precision)"))
  (returns (IsArrived :type Boolean))
  (return (>= Length (`SplineComponent.GetSplineLength` (`self.Spline`)))))

(fn `UserConstructionScript`)