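; Snitch actor Blueprint with movement logic that reacts to walls and the player's proximity, though Tick is empty and that logic is disconnected, so it never runs.
; GetVariaties derives trace endpoints, player distance flags and a look-at rotation.
; The unwired graph turns on forward trace hits, boosts forward movement within encounter range, and applies a one-shot look-at-plus-flip rotation when the player closes in.
; The sideways teleport branch is unfinished.
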(event `self.ReceiveTick`
  (params (DeltaSeconds :type "Float (single-precision)")))

(fn `GetVariaties`
  (bind _returnvalue (`self.K2_GetActorLocation`))
  (bind _returnvalue_2 (`self.K2_GetActorLocation` (`GameplayStatics.GetPlayerCharacter` 0)))
  (`|ExecutionSequence`
    (:`then_0`
      ;[1 1 1] GetForwardVector
      (bind _output_get (set `self.UnitForwardVector` (`self.GetActorForwardVector`)))
      (set `self.ForwardVector` (+ (* _output_get (`self.FVRate`)) (`self.K2_GetActorLocation`))))
    (:`then_1`
      ;[1 1 1] GetRightVector
      (bind _output_get_2 (set `self.UnitRightVector` (`self.GetActorRightVector`)))
      (set `self.RightVector` (+ (* _output_get_2 (`self.RVRate`)) (`self.K2_GetActorLocation`))))
    (:`then_2`
      ;[1 1 1] GetEtc.
      (`KismetSystemLibrary.LineTraceSingle` _returnvalue _returnvalue_2 "TraceTypeQuery1" true)
      (set `self.LookRotate` (`KismetMathLibrary.FindLookAtRotation` _returnvalue _returnvalue_2))
      (bind _output_get_3 (set `self.PVectorLength` (`KismetMathLibrary.VSize` (- (`self.K2_GetActorLocation`) (`self.K2_GetActorLocation` (`GameplayStatics.GetPlayerCharacter` 0))))))
      (set `self.Encount` (<= _output_get_3 (`self.EncountDistance`)))
      (set `self.PlayerClosing` (<= _output_get_3 (`self.LookBackDistance`))))))

(fn `UserConstructionScript`)