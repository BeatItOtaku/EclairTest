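; Door actor Blueprint that opens an animated door when all of its linked switches are on.
; BeginPlay caches the skeletal mesh's DoorAnimBP anim instance.
; Each Tick multiplies +1 or -1 per switch in SwitchActors, stopping at the first switch that is off, and writes the result to the anim instance's IsOpen flag.
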(event `self.ReceiveBeginPlay`
  (bind _asdoor_anim_bp (cast `/Game/Fbx/Door/DoorAnimBP` (`SkeletalMeshComponent.GetAnimInstance` (`self.SkeletalMeshComponent`))))
  (set `self.DoorAnimBP` _asdoor_anim_bp))

(event `self.ReceiveTick`
  (params (DeltaSeconds :type "Float (single-precision)"))
  (set `self.SwitchOnCount` 1)
  (for _array_element (`self.SwitchActors`)
    (bind _output_get (set `self.SwitchOnCount` (* (`self.SwitchOnCount`) (`KismetMathLibrary.SelectInt` 1 -1 (`/Game/Blueprints/SwitchActor_Blueprint.SwitchOn` _array_element)))))
    (if (not (> _output_get 0))
      (break)))
  (set `/Game/Fbx/Door/DoorAnimBP.IsOpen` (> (`self.SwitchOnCount`) 0) (`self.DoorAnimBP`)))

(fn `UserConstructionScript`)