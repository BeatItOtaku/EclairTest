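; Kurage actor that drifts along its local Z axis and starts sinking once the player character hits it.
; A static mesh hit from a ThirdPersonCharacter sets OnPlayer, which is never cleared here.
; Each tick moves it by the sine of the frame delta, a small steady rise rather than a bob, or by a fixed downward step once flagged.
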(event OnComponentHit(StaticMeshComponent)
  (params (HitComponent :type Primitive%20Component%20Object%20Reference) (OtherActor :type Actor%20Object%20Reference) (OtherComp :type Primitive%20Component%20Object%20Reference) (NormalImpulse :type Vector :default "0, 0, 0") (Hit :type Hit%20Result%20Structure%20%28by%20ref%29))
  (Utilities|Casting|CastToThirdPersonCharacter OtherActor)
  (Variables|Default|SetOnPlayer true))

(event EventTick
  (params (DeltaSeconds :type Float%20%28single-precision%29))
  (if (Variables|Default|GetOnPlayer)
    (Class|Actor|AddActorLocalTransform (Math|Transform|MakeTransform (Math|Vector|MakeVector 0.0 0.0 -0.5) "0, 0, 0" "1,1,1") false false)
    (else
      (Class|Actor|AddActorLocalTransform (Math|Transform|MakeTransform (Math|Vector|MakeVector 0.0 0.0 (|(Sin(DeltaSeconds)) DeltaSeconds)) "0, 0, 0" "1,1,1") false false))))

(fn ConstructionScript)