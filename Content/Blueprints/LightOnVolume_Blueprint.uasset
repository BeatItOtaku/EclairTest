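; Trigger volume Blueprint that fades in a directional light when the third-person character enters it.
; BeginPlay sets the light to zero intensity.
; The collision overlap sets PlayerOverlap from the event's FromSweep value rather than a literal true, and no end-overlap handler exists.
; While the flag is true, Tick eases the intensity toward the target with a fixed-alpha Lerp, so the fade speed depends on frame rate.
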(event `self.ReceiveBeginPlay`
  (`LightComponent.SetIntensity` (`Light.LightComponent` (`self.DirectionalLight`)) 0.0))

(event `self.ReceiveTick`
  (params (DeltaSeconds :type "Float (single-precision)"))
  (if (`self.PlayerOverlap`)
    (bind _output_get (set `self.CurrentIntensity` (`KismetMathLibrary.Lerp` (`self.CurrentIntensity`) (`self.Intensity`) 0.01)))
    (`LightComponent.SetIntensity` (`Light.LightComponent` (`self.DirectionalLight`)) _output_get)))

(event `self.Collision.OnComponentBeginOverlap`
  (params (OverlappedComponent :type "PrimitiveComponent Object Reference") (OtherActor :type "Actor Object Reference") (OtherComp :type "PrimitiveComponent Object Reference") (OtherBodyIndex :type Integer) (bFromSweep :type Boolean) (SweepResult :type "HitResult Structure (by ref)"))
  (cast `/Game/ThirdPersonBP/Blueprints/ThirdPersonCharacter` OtherActor)
  (set `self.PlayerOverlap` bFromSweep))

(fn `UserConstructionScript`)