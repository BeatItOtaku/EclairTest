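; Kurage (jellyfish) actor that destroys itself after something stays above it for more than three seconds.
; Each tick a box trace along its up vector checks the configured object types and stores any blocking hit as OnEclair.
; OnEclairTime accumulates while that flag is set and resets otherwise, with debug drawing and a printout of the timer left on.
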(event `self.ReceiveTick`
  (params (DeltaSeconds :type "Float (single-precision)"))
  (bind _returnvalue (`self.K2_GetActorLocation`))
  (bind _oneclairtime (`self.OnEclairTime`))
  (if (`self.OnEclair`)
    (set `self.OnEclairTime` (+ DeltaSeconds (`self.OnEclairTime`)))
    (else
      (set `self.OnEclairTime` 0.0)))
  (bind _outhit (`KismetSystemLibrary.BoxTraceSingleForObjects` :`Start` _returnvalue :`End` (+ _returnvalue (* (`self.GetActorUpVector`) 200.0)) :`HalfSize` (250.0 250.0 0.0) :`ObjectTypes` (`self.RayHitObjects`) :`DrawDebugType` "ForOneFrame"))
  (bind _output_get (set `self.OnEclair` (`GameplayStatics.BreakHitResult` _outhit)))
  (`KismetSystemLibrary.PrintString` (`KismetStringLibrary.Conv_DoubleToString` _oneclairtime))
  (if (> _oneclairtime 3.0)
    (`self.K2_DestroyActor`)))

(fn `UserConstructionScript`)